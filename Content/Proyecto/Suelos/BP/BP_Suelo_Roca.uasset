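; Rock floor tile for a three-lane endless runner starring an astronaut.
; On BeginPlay, each lane rolls a random spawn of obstacle, coin, oxygen, gem or nothing.
; When the astronaut overlaps its collision, it has the game mode spawn another tile, adds multiplied run points, calls Breath, slightly raises clamped walk speed, then destroys itself after a short delay.
; SetSpawn, SpawnObstacle and SpawnObjetos logic is left unwired.
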(event OnComponentBeginOverlap(Collision)
  (params (OverlappedComponent :type Primitive%20Component%20Object%20Reference) (OtherActor :type Actor%20Object%20Reference) (OtherComp :type Primitive%20Component%20Object%20Reference) (OtherBodyIndex :type Integer) (bFromSweep :type Boolean) (SweepResult :type Hit%20Result%20Structure%20%28by%20ref%29))
  (Utilities|Casting|CastToAstronauta OtherActor)
  (bind _asthird_person_game_mode (Utilities|Casting|CastToThirdPersonGameMode (Game|GetGameMode)))
  (Default|SpawnSuelo _asthird_person_game_mode)
  (bind _asthird_person_game_mode_2 (Utilities|Casting|CastToThirdPersonGameMode (Game|GetGameMode)))
  (Variables|/Game/ThirdPersonBP/Blueprints/ThirdPersonGameMode.ThirdPersonGameMode_C|SetPuntosCarrera _asthird_person_game_mode_2 (+ (* 1 (Variables|/Game/ThirdPersonBP/Blueprints/ThirdPersonGameMode.ThirdPersonGameMode_C|GetMultiplicador_puntos _asthird_person_game_mode_2)) (Variables|/Game/ThirdPersonBP/Blueprints/ThirdPersonGameMode.ThirdPersonGameMode_C|GetPuntosCarrera _asthird_person_game_mode_2)))
  (bind _asastronauta (Utilities|Casting|CastToAstronauta (Game|GetPlayerCharacter 0)))
  (Default|Breath _asastronauta)
  (bind _asastronauta_2 (Utilities|Casting|CastToAstronauta (Game|GetPlayerCharacter 0)))
  (Variables|/Script/Engine.CharacterMovementComponent|SetMaxWalkSpeed (Variables|/Script/Engine.Character|GetCharacterMovement _asastronauta_2) (Math|Float|Clamp(Float) (* 1.0025 (Variables|/Script/Engine.CharacterMovementComponent|GetMaxWalkSpeed (Variables|/Script/Engine.Character|GetCharacterMovement _asastronauta_2))) 1e+03 5e+03))
  (Utilities|FlowControl|Delay 0.8)
  (Actor|DestroyActor))

(event EventBeginPlay
  (CallFunction|SpawnObstacleLeft)
  (CallFunction|SpawnObstacleMiddle)
  (CallFunction|SpawnObstacleRight))

(fn ConstructionScript)

(fn SetSpawn
  ;[1 1 1] Coge las cordenadas de los spawn point y las guarda en un array
  (Variables|Default|SetSpawnPoints (Utilities|Array|MakeArray (Transformation|GetRelativeTransform (Variables|Default|GetSpawn)) (Transformation|GetRelativeTransform (Variables|Default|GetSpawn_Left)) (Transformation|GetRelativeTransform (Variables|Default|GetSpawn_Right)) (Transformation|GetRelativeTransform (Variables|Default|GetSpawn_Left0)) (Transformation|GetRelativeTransform (Variables|Default|GetSpawn_Right0)) (Transformation|GetRelativeTransform (Variables|Default|GetSpawn0)))))

(fn SpawnObstacle
  (bind _spawnpoints (Variables|Default|GetSpawnPoints))
  ;[1 1 1] Crea obstaculos en una de las ubicaciones del array (escogida random)
  (AddComponent|AddChildActorComponent false (Utilities|Array|Get(acopy) _spawnpoints (Math|Random|RandomIntegerinRange 0 (Utilities|Array|LastIndex _spawnpoints)))))

(fn SpawnObjetos)

(fn SpawnObstacleLeft
  (bind _left (Variables|Default|GetLeft))
  ;[1 1 1] Izquierda
  (switch int (Math|Random|RandomIntegerinRange 0 (Variables|Default|GetMax_Rand_Obstacle))
    (:1
      (Game|SpawnActorfromClass 0 (Transformation|GetWorldTransform _left) "Undefined" 0 0))
    (:2
      (Game|SpawnActorfromClass "/Game/Proyecto/Props/Obstaculo_Grande_I.Obstaculo_Grande_I_C" (Transformation|GetWorldTransform _left) "Undefined" 0 0))
    (:3
      (Game|SpawnActorfromClass "/Game/Proyecto/Props/MonedaBasica.MonedaBasica_C" (Transformation|GetWorldTransform _left) "Undefined" 0 0))
    (:4
      (Game|SpawnActorfromClass "/Game/Proyecto/Props/Oxigeno.Oxigeno_C" (Transformation|GetWorldTransform _left) "Undefined" 0 0))
    (:5
      (Game|SpawnActorfromClass "/Game/Proyecto/Props/Gemas.Gemas_C" (Transformation|GetWorldTransform _left) "Undefined" 0 0))
    (:6
      (Game|SpawnActorfromClass "/Game/Proyecto/Props/MonedaBasica.MonedaBasica_C" (Transformation|GetWorldTransform _left) "Undefined" 0 0))
    (:7
      (Game|SpawnActorfromClass "/Game/Proyecto/Props/Obstaculo_Grande_I.Obstaculo_Grande_I_C" (Transformation|GetWorldTransform _left) "Undefined" 0 0))
    (:8
      (Game|SpawnActorfromClass 0 (Transformation|GetWorldTransform _left) "Undefined" 0 0))))

(fn SpawnObstacleMiddle
  (bind _middle (Variables|Default|GetMiddle))
  ;[1 1 1] Medio
  (switch int (Math|Random|RandomIntegerinRange 0 (Variables|Default|GetMax_Rand_Obstacle))
    (:1
      (Game|SpawnActorfromClass 0 (Transformation|GetWorldTransform _middle) "Undefined" 0 0))
    (:2
      (Game|SpawnActorfromClass "/Game/Proyecto/Props/Obstaculo_Grande_I.Obstaculo_Grande_I_C" (Transformation|GetWorldTransform _middle) "Undefined" 0 0))
    (:3
      (Game|SpawnActorfromClass "/Game/Proyecto/Props/MonedaBasica.MonedaBasica_C" (Transformation|GetWorldTransform _middle) "Undefined" 0 0))
    (:4
      (Game|SpawnActorfromClass "/Game/Proyecto/Props/Oxigeno.Oxigeno_C" (Transformation|GetWorldTransform _middle) "Undefined" 0 0))
    (:5
      (Game|SpawnActorfromClass "/Game/Proyecto/Props/Gemas.Gemas_C" (Transformation|GetWorldTransform _middle) "Undefined" 0 0))
    (:6
      (Game|SpawnActorfromClass "/Game/Proyecto/Props/MonedaBasica.MonedaBasica_C" (Transformation|GetWorldTransform _middle) "Undefined" 0 0))
    (:7
      (Game|SpawnActorfromClass "/Game/Proyecto/Props/Obstaculo_Grande_I.Obstaculo_Grande_I_C" (Transformation|GetWorldTransform _middle) "Undefined" 0 0))
    (:8
      (Game|SpawnActorfromClass 0 (Transformation|GetWorldTransform _middle) "Undefined" 0 0))))

(fn SpawnObstacleRight
  (bind _rigth (Variables|Default|GetRigth))
  ;[1 1 1] Derecha
  (switch int (Math|Random|RandomIntegerinRange 0 (Variables|Default|GetMax_Rand_Obstacle))
    (:1
      (Game|SpawnActorfromClass 0 (Transformation|GetWorldTransform _rigth) "Undefined" 0 0))
    (:2
      (Game|SpawnActorfromClass "/Game/Proyecto/Props/Obstaculo_Grande_I.Obstaculo_Grande_I_C" (Transformation|GetWorldTransform _rigth) "Undefined" 0 0))
    (:3
      (Game|SpawnActorfromClass "/Game/Proyecto/Props/MonedaBasica.MonedaBasica_C" (Transformation|GetWorldTransform _rigth) "Undefined" 0 0))
    (:4
      (Game|SpawnActorfromClass "/Game/Proyecto/Props/Oxigeno.Oxigeno_C" (Transformation|GetWorldTransform _rigth) "Undefined" 0 0))
    (:5
      (Game|SpawnActorfromClass "/Game/Proyecto/Props/Gemas.Gemas_C" (Transformation|GetWorldTransform _rigth) "Undefined" 0 0))
    (:6
      (Game|SpawnActorfromClass "/Game/Proyecto/Props/MonedaBasica.MonedaBasica_C" (Transformation|GetWorldTransform _rigth) "Undefined" 0 0))
    (:7
      (Game|SpawnActorfromClass "/Game/Proyecto/Props/Obstaculo_Grande_I.Obstaculo_Grande_I_C" (Transformation|GetWorldTransform _rigth) "Undefined" 0 0))
    (:8
      (Game|SpawnActorfromClass 0 (Transformation|GetWorldTransform _rigth) "Undefined" 0 0))))