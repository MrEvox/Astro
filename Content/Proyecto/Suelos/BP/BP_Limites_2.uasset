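; BP_Limites_2 is a boundary segment that requests the next one from the game mode as the player advances.
; On BeginPlay a random four-way switch sets the LimiteL mesh and material, though every branch currently assigns the same Limite02 mesh and Limite2_m2 material.
; When an Astronauta overlaps its Collision component, it casts the game mode to ThirdPersonGameMode and calls SpawnLimite.
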(event OnComponentBeginOverlap(Collision)
  (params (OverlappedComponent :type Primitive%20Component%20Object%20Reference) (OtherActor :type Actor%20Object%20Reference) (OtherComp :type Primitive%20Component%20Object%20Reference) (OtherBodyIndex :type Integer) (bFromSweep :type Boolean) (SweepResult :type Hit%20Result%20Structure%20%28by%20ref%29))
  (Utilities|Casting|CastToAstronauta OtherActor)
  (bind _asthird_person_game_mode (Utilities|Casting|CastToThirdPersonGameMode (Game|GetGameMode)))
  (Default|SpawnLimite _asthird_person_game_mode))

(event EventBeginPlay
  (bind _limitel (Variables|Default|GetLimiteL))
  (switch int (Math|Random|RandomIntegerinRange 0 3)
    (:0
      (Components|StaticMesh|SetStaticMesh _limitel "/Game/Proyecto/Assets_Definitivos/Limites/limite02_M2/limite02_M2_LP_chino_2_.limite02_M2_LP_chino_2_")
      (Rendering|Material|SetMaterial _limitel 0 "/Game/Proyecto/Assets_Definitivos/Limites/limite02_M2/limite2_m2.limite2_m2"))
    (:1
      (Components|StaticMesh|SetStaticMesh _limitel "/Game/Proyecto/Assets_Definitivos/Limites/limite02_M2/limite02_M2_LP_chino_2_.limite02_M2_LP_chino_2_")
      (Rendering|Material|SetMaterial _limitel 0 "/Game/Proyecto/Assets_Definitivos/Limites/limite02_M2/limite2_m2.limite2_m2"))
    (:2
      (Components|StaticMesh|SetStaticMesh _limitel "/Game/Proyecto/Assets_Definitivos/Limites/limite02_M2/limite02_M2_LP_chino_2_.limite02_M2_LP_chino_2_")
      (Rendering|Material|SetMaterial _limitel 0 "/Game/Proyecto/Assets_Definitivos/Limites/limite02_M2/limite2_m2.limite2_m2"))
    (:3
      (Components|StaticMesh|SetStaticMesh _limitel "/Game/Proyecto/Assets_Definitivos/Limites/limite02_M2/limite02_M2_LP_chino_2_.limite02_M2_LP_chino_2_")
      (Rendering|Material|SetMaterial _limitel 0 "/Game/Proyecto/Assets_Definitivos/Limites/limite02_M2/limite2_m2.limite2_m2"))))

(fn ConstructionScript)