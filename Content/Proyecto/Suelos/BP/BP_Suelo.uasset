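; Floor tile for an endless runner that chains the track as the Astronauta runs over it.
; Construction caches six spawn-point transforms and adds one random obstacle child actor at one of them.
; Collision overlap has ThirdPersonGameMode spawn the next tile, adds multiplied points, calls Breath and slightly raises clamped walk speed, then destroys the tile after a delay.
; SpawnObjetos is empty, leaving its lane-based collectible logic disconnected.
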(event OnComponentBeginOverlap(Collision)
  (params (OverlappedComponent :type Primitive%20Component%20Object%20Reference) (OtherActor :type Actor%20Object%20Reference) (OtherComp :type Primitive%20Component%20Object%20Reference) (OtherBodyIndex :type Integer) (bFromSweep :type Boolean) (SweepResult :type Hit%20Result%20Structure%20%28by%20ref%29))
  (Utilities|Casting|CastToAstronauta OtherActor)
  (bind _asthird_person_game_mode (Utilities|Casting|CastToThirdPersonGameMode (Game|GetGameMode)))
  (Default|SpawnSuelo _asthird_person_game_mode)
  (bind _asthird_person_game_mode_2 (Utilities|Casting|CastToThirdPersonGameMode (Game|GetGameMode)))
  (Variables|/Game/ThirdPersonBP/Blueprints/ThirdPersonGameMode.ThirdPersonGameMode_C|SetPuntosCarrera _asthird_person_game_mode_2 (+ (* 1 (Variables|/Game/ThirdPersonBP/Blueprints/ThirdPersonGameMode.ThirdPersonGameMode_C|GetMultiplicador_puntos _asthird_person_game_mode_2)) (Variables|/Game/ThirdPersonBP/Blueprints/ThirdPersonGameMode.ThirdPersonGameMode_C|GetPuntosCarrera _asthird_person_game_mode_2)))
  (bind _asastronauta (Utilities|Casting|CastToAstronauta (Game|GetPlayerCharacter 0)))
  (Default|Breath _asastronauta)
  (bind _asastronauta_2 (Utilities|Casting|CastToAstronauta (Game|GetPlayerCharacter 0)))
  (Variables|/Script/Engine.CharacterMovementComponent|SetMaxWalkSpeed (Variables|/Script/Engine.Character|GetCharacterMovement _asastronauta_2) (Math|Float|Clamp(Float) (* 1.0025 (Variables|/Script/Engine.CharacterMovementComponent|GetMaxWalkSpeed (Variables|/Script/Engine.Character|GetCharacterMovement _asastronauta_2))) 1e+03 5e+03))
  (Utilities|FlowControl|Delay 0.8)
  (Actor|DestroyActor))

(event EventBeginPlay)

(event Collision|EventActorBeginOverlap
  (params (OtherActor :type Actor%20Object%20Reference)))

(event EventTick
  (params (DeltaSeconds :type Float%20%28single-precision%29)))

(fn ConstructionScript
  (CallFunction|SetSpawn)
  (CallFunction|SpawnObstacle))

(fn SetSpawn
  ;[1 1 1] Coge las cordenadas de los spawn point y las guarda en un array
  (Variables|Default|SetSpawnPoints (Utilities|Array|MakeArray (Transformation|GetRelativeTransform (Variables|Default|GetSpawn)) (Transformation|GetRelativeTransform (Variables|Default|GetSpawn_Left)) (Transformation|GetRelativeTransform (Variables|Default|GetSpawn_Right)) (Transformation|GetRelativeTransform (Variables|Default|GetSpawn_Left0)) (Transformation|GetRelativeTransform (Variables|Default|GetSpawn_Right0)) (Transformation|GetRelativeTransform (Variables|Default|GetSpawn0)))))

(fn SpawnObstacle
  (bind _spawnpoints (Variables|Default|GetSpawnPoints))
  (bind _returnvalue (Utilities|Array|LastIndex _spawnpoints))
  (bind _returnvalue_2 (Math|Random|RandomIntegerinRange 0 _returnvalue))
  (bind _output (Utilities|Array|Get(acopy) _spawnpoints _returnvalue_2))
  ;[1 1 1] Crea obstaculos en una de las ubicaciones del array (escogida random)
  (switch int (Math|Integer|Clamp(Integer) (Math|Random|RandomInteger 5) 0 5)
    (:0
      (AddComponent|AddChildActorComponent false _output))
    (:1
      (AddComponent|AddChildActorComponent false _output))
    (:2
      (AddComponent|AddChildActorComponent false _output))
    (:3
      (AddComponent|AddChildActorComponent false _output))
    (:4
      (AddComponent|AddChildActorComponent false _output))))

(fn SpawnObjetos)