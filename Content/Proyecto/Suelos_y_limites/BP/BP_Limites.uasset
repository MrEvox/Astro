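; Boundary segment (Limite) with left and right meshes that requests the next segment as the astronaut reaches it.
; On BeginPlay each side makes a random four-way pick of mesh and material, though every option currently assigns the same Limite01 mesh and material.
; When an Astronauta begins overlapping the Collision component, it calls SpawnLimite on the ThirdPersonGameMode, chaining boundaries during play.
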(event OnComponentBeginOverlap(Collision)
  (params (OverlappedComponent :type Primitive%20Component%20Object%20Reference) (OtherActor :type Actor%20Object%20Reference) (OtherComp :type Primitive%20Component%20Object%20Reference) (OtherBodyIndex :type Integer) (bFromSweep :type Boolean) (SweepResult :type Hit%20Result%20Structure%20%28by%20ref%29))
  (Utilities|Casting|CastToAstronauta OtherActor)
  (bind _asthird_person_game_mode (Utilities|Casting|CastToThirdPersonGameMode (Game|GetGameMode)))
  (Default|SpawnLimite _asthird_person_game_mode))

(event EventBeginPlay
  (bind _limitel (Variables|Default|GetLimiteL))
  (bind _limiter (Variables|Default|GetLimiteR))
  (switch int (Math|Random|RandomIntegerinRange 0 3)
    (:0
      (Components|StaticMesh|SetStaticMesh _limitel "/Game/Proyecto/Suelos_y_limites/assets/limites/limite01_M1/limite01.limite01")
      (Rendering|Material|SetMaterial _limitel 0 "/Game/Proyecto/Suelos_y_limites/assets/limites/limite01_M1/limite_1_m1.limite_1_m1"))
    (:1
      (Components|StaticMesh|SetStaticMesh _limitel "/Game/Proyecto/Suelos_y_limites/assets/limites/limite01_M1/limite01.limite01")
      (Rendering|Material|SetMaterial _limitel 0 "/Game/Proyecto/Suelos_y_limites/assets/limites/limite01_M1/limite_1_m1.limite_1_m1"))
    (:2
      (Components|StaticMesh|SetStaticMesh _limitel "/Game/Proyecto/Suelos_y_limites/assets/limites/limite01_M1/limite01.limite01")
      (Rendering|Material|SetMaterial _limitel 0 "/Game/Proyecto/Suelos_y_limites/assets/limites/limite01_M1/limite_1_m1.limite_1_m1"))
    (:3
      (Components|StaticMesh|SetStaticMesh _limitel "/Game/Proyecto/Suelos_y_limites/assets/limites/limite01_M1/limite01.limite01")
      (Rendering|Material|SetMaterial _limitel 0 "/Game/Proyecto/Suelos_y_limites/assets/limites/limite01_M1/limite_1_m1.limite_1_m1")))
  (switch int (Math|Random|RandomIntegerinRange 0 3)
    (:0
      (Components|StaticMesh|SetStaticMesh _limiter "/Game/Proyecto/Suelos_y_limites/assets/limites/limite01_M1/limite01.limite01")
      (Rendering|Material|SetMaterial _limiter 0 "/Game/Proyecto/Suelos_y_limites/assets/limites/limite01_M1/limite_1_m1.limite_1_m1"))
    (:1
      (Components|StaticMesh|SetStaticMesh _limiter "/Game/Proyecto/Suelos_y_limites/assets/limites/limite01_M1/limite01.limite01")
      (Rendering|Material|SetMaterial _limiter 0 "/Game/Proyecto/Suelos_y_limites/assets/limites/limite01_M1/limite_1_m1.limite_1_m1"))
    (:2
      (Components|StaticMesh|SetStaticMesh _limiter "/Game/Proyecto/Suelos_y_limites/assets/limites/limite01_M1/limite01.limite01")
      (Rendering|Material|SetMaterial _limiter 0 "/Game/Proyecto/Suelos_y_limites/assets/limites/limite01_M1/limite_1_m1.limite_1_m1"))
    (:3
      (Components|StaticMesh|SetStaticMesh _limiter "/Game/Proyecto/Suelos_y_limites/assets/limites/limite01_M1/limite01.limite01")
      (Rendering|Material|SetMaterial _limiter 0 "/Game/Proyecto/Suelos_y_limites/assets/limites/limite01_M1/limite_1_m1.limite_1_m1"))))

(fn ConstructionScript)