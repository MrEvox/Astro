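; Three-lane floor tile for an endless runner that picks one of four mesh variants at BeginPlay and populates lanes to match.
; Per-lane functions randomly spawn obstacles, pickups and worms, while the last variant gets only a jump coin trail.
; When the Astronauta hits the Collision trigger, the game mode spawns the next tile and adds score, the player breathes and speeds up, and the tile self-destructs after a delay.
; Touching the Caida volume kills the player.
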(event OnComponentBeginOverlap(Collision)
  (params (OverlappedComponent :type Primitive%20Component%20Object%20Reference) (OtherActor :type Actor%20Object%20Reference) (OtherComp :type Primitive%20Component%20Object%20Reference) (OtherBodyIndex :type Integer) (bFromSweep :type Boolean) (SweepResult :type Hit%20Result%20Structure%20%28by%20ref%29))
  (Utilities|Casting|CastToAstronauta OtherActor)
  (bind _asthird_person_game_mode (Utilities|Casting|CastToThirdPersonGameMode (Game|GetGameMode)))
  (Default|SpawnSuelo2 _asthird_person_game_mode)
  (bind _asthird_person_game_mode_2 (Utilities|Casting|CastToThirdPersonGameMode (Game|GetGameMode)))
  (Variables|/Game/ThirdPersonBP/Blueprints/ThirdPersonGameMode.ThirdPersonGameMode_C|SetPuntosCarrera _asthird_person_game_mode_2 (+ (* 1 (Variables|/Game/ThirdPersonBP/Blueprints/ThirdPersonGameMode.ThirdPersonGameMode_C|GetMultiplicador_puntos _asthird_person_game_mode_2)) (Variables|/Game/ThirdPersonBP/Blueprints/ThirdPersonGameMode.ThirdPersonGameMode_C|GetPuntosCarrera _asthird_person_game_mode_2)))
  (bind _asastronauta (Utilities|Casting|CastToAstronauta (Game|GetPlayerCharacter 0)))
  (Default|Breath _asastronauta)
  (bind _asastronauta_2 (Utilities|Casting|CastToAstronauta (Game|GetPlayerCharacter 0)))
  (Variables|/Script/Engine.CharacterMovementComponent|SetMaxWalkSpeed (Variables|/Script/Engine.Character|GetCharacterMovement _asastronauta_2) (Math|Float|Clamp(Float) (* 1.0025 (Variables|/Script/Engine.CharacterMovementComponent|GetMaxWalkSpeed (Variables|/Script/Engine.Character|GetCharacterMovement _asastronauta_2))) 1e+03 5e+03))
  (Utilities|FlowControl|Delay 0.8)
  (Actor|DestroyActor))

(event OnComponentBeginOverlap(Caida)
  (params (OverlappedComponent :type Primitive%20Component%20Object%20Reference) (OtherActor :type Actor%20Object%20Reference) (OtherComp :type Primitive%20Component%20Object%20Reference) (OtherBodyIndex :type Integer) (bFromSweep :type Boolean) (SweepResult :type Hit%20Result%20Structure%20%28by%20ref%29))
  (bind _asastronauta (Utilities|Casting|CastToAstronauta OtherActor))
  (Variables|/Game/ThirdPersonBP/Blueprints/Astronauta.Astronauta_C|SetIsDead _asastronauta true))

(event EventBeginPlay
  (bind _cube (Variables|Default|GetCube))
  (bind _cube_2 (Variables|Default|GetCube))
  (switch int (Math|Random|RandomIntegerinRange 0 3)
    (:0
      (Components|StaticMesh|SetStaticMesh _cube_2 "/Game/Proyecto/Suelos_y_limites/assets/suelos/Suelos_Mundo1/Base_3carriles/Base3carriles_lowpoly.Base3carriles_lowpoly")
      (Rendering|Material|SetMaterial _cube 0 "/Game/Proyecto/Suelos_y_limites/assets/suelos/Suelos_Mundo1/Base_3carriles/Base_3carriles_mat_m2.Base_3carriles_mat_m2")
      (CallFunction|SpawnObstacleMiddle)
      (CallFunction|SpawnObstacleRight)
      (CallFunction|SpawnObstacleLeft))
    (:1
      (Components|StaticMesh|SetStaticMesh _cube_2 "/Game/Proyecto/Suelos_y_limites/assets/suelos/Suelos_Mundo1/3carriles_01/3carriles_01_LP.3carriles_01_LP")
      (Rendering|Material|SetMaterial _cube 0 "/Game/Proyecto/Suelos_y_limites/assets/suelos/Suelos_Mundo1/3carriles_01/3carriles_01_mat_m2.3carriles_01_mat_m2")
      (CallFunction|SpawnObstacleMiddle)
      (CallFunction|SpawnObstacleLeft))
    (:2
      (Components|StaticMesh|SetStaticMesh _cube_2 "/Game/Proyecto/Suelos_y_limites/assets/suelos/Suelos_Mundo1/3carriles_02/3carriles_02_LP.3carriles_02_LP")
      (Rendering|Material|SetMaterial _cube 0 "/Game/Proyecto/Suelos_y_limites/assets/suelos/Suelos_Mundo1/3carriles_02/3carriles_02_mat_m2.3carriles_02_mat_m2")
      (CallFunction|SpawnObstacleRight)
      (CallFunction|SpawnObstacleLeft))
    (:3
      (Components|StaticMesh|SetStaticMesh _cube_2 "/Game/Proyecto/Suelos_y_limites/assets/suelos/Suelos_Mundo1/3carriles_03/3carriles_03_LP.3carriles_03_LP")
      (Rendering|Material|SetMaterial _cube 0 "/Game/Proyecto/Suelos_y_limites/assets/suelos/Suelos_Mundo1/3carriles_03/3carriles_03_mar_m2.3carriles_03_mar_m2")
      (CallFunction|SpawnSaltoMonedas))))

(fn ConstructionScript)

(fn SetSpawn
  ;[1 1 1] Coge las cordenadas de los spawn point y las guarda en un array
  (Variables|Default|SetSpawnPoints (Utilities|Array|MakeArray (Transformation|GetRelativeTransform (Variables|Default|GetSpawn)) (Transformation|GetRelativeTransform (Variables|Default|GetSpawn_Left)) (Transformation|GetRelativeTransform (Variables|Default|GetSpawn_Right)) (Transformation|GetRelativeTransform (Variables|Default|GetSpawn_Left0)) (Transformation|GetRelativeTransform (Variables|Default|GetSpawn_Right0)) (Transformation|GetRelativeTransform (Variables|Default|GetSpawn0)))))

(fn SpawnObstacle
  (bind _spawnpoints (Variables|Default|GetSpawnPoints))
  ;[1 1 1] Crea obstaculos en una de las ubicaciones del array (escogida random)
  (AddComponent|AddChildActorComponent false (Utilities|Array|Get(acopy) _spawnpoints (Math|Random|RandomIntegerinRange 0 (Utilities|Array|LastIndex _spawnpoints)))))

(fn SpawnObjetos)

(fn SpawnObstacleLeft
  (bind _left (Variables|Default|GetLeft))
  (bind _returnvalue (Transformation|GetWorldTransform _left))
  (bind _returnvalue_2 (Transformation|GetWorldTransform _left))
  ;[1 1 1] Izquierda
  (switch int (Math|Random|RandomIntegerinRange 0 (Variables|Default|GetMax_Rand_Obstacle))
    (:0
      (Game|SpawnActorfromClass "/Game/Proyecto/Props/Carril_Moneda.Carril_Moneda_C" (Transformation|GetWorldTransform _left) "Undefined" 0 0))
    (:1
      (Game|SpawnActorfromClass "/Game/Proyecto/Props/Oxigeno.Oxigeno_C" (Transformation|GetWorldTransform _left) "Undefined" 0 0))
    (:2
      (bind _returnvalue_3 (Game|SpawnActorfromClass "/Game/Proyecto/Obstaculos/BP/Obstaculo_Piedra.Obstaculo_Piedra_C" (Transformation|GetWorldTransform _left) "Undefined" 0 0))
      (Rendering|Material|SetMaterial (Variables|/Game/Proyecto/Obstaculos/BP/Obstaculo_Piedra.Obstaculo_Piedra_C|GetCube _returnvalue_3) 0 "/Game/Proyecto/Obstaculos/Assets/Obstaculo1_rocas/Obstaculo_Piedras_mat_2.Obstaculo_Piedras_mat_2"))
    (:3
      (Game|SpawnActorfromClass "/Game/Proyecto/Props/Carril_Moneda.Carril_Moneda_C" (Transformation|GetWorldTransform _left) "Undefined" 0 0))
    (:4
      (Game|SpawnActorfromClass "/Game/Proyecto/Obstaculos/BP/Obstaculo_Cactus.Obstaculo_Cactus_C" (Transformation|GetWorldTransform _left) "Undefined" 0 0))
    (:5
      (Game|SpawnActorfromClass "/Game/Proyecto/Obstaculos/BP/Obstaculo_Agacharse.Obstaculo_Agacharse_C" _returnvalue_2 "Undefined" 0 0)
      (switch int (Math|Random|RandomIntegerinRange 0 3)
        (:0
          (Game|SpawnActorfromClass "/Game/Proyecto/Props/Carril_Moneda_Oxigeno.Carril_Moneda_Oxigeno_C" _returnvalue_2 "Undefined" 0 0))
        (:1
          (Game|SpawnActorfromClass "/Game/Proyecto/Props/Carril_Moneda_XL.Carril_Moneda_XL_C" _returnvalue_2 "Undefined" 0 0))
        (:2
          (Game|SpawnActorfromClass "/Game/Proyecto/Props/Gemas.Gemas_C" _returnvalue_2 "Undefined" 0 0))))
    (:6
      (Game|SpawnActorfromClass "/Game/Proyecto/Obstaculos/BP/Obstaculo_Cactus.Obstaculo_Cactus_C" (Transformation|GetWorldTransform _left) "Undefined" 0 0))
    (:7
      (Game|SpawnActorfromClass "/Game/Proyecto/Props/Gemas.Gemas_C" (Transformation|GetWorldTransform _left) "Undefined" 0 0))
    (:8
      (Game|SpawnActorfromClass "/Game/Proyecto/Obstaculos/BP/Gusano1-Izquierda.Gusano1-Izquierda_C" (Transformation|GetWorldTransform _left) "Undefined" 0 0))
    (:9
      (switch int (Math|Random|RandomIntegerinRange 0 1)
        (:0
          (Game|SpawnActorfromClass "/Game/Proyecto/PowerUps/BP/Desfasador.Desfasador_C" _returnvalue "Undefined" 0 0))
        (:1
          (Game|SpawnActorfromClass "/Game/Proyecto/Obstaculos/BP/Gusano1-Derecha.Gusano1-Derecha_C" _returnvalue "Undefined" 0 0))))))

(fn SpawnObstacleMiddle
  (bind _middle (Variables|Default|GetMiddle))
  (bind _returnvalue (Transformation|GetWorldTransform _middle))
  ;[1 1 1] Medio
  (switch int (Math|Random|RandomIntegerinRange 0 (Variables|Default|GetMax_Rand_Obstacle))
    (:0
      (bind _returnvalue_2 (Game|SpawnActorfromClass "/Game/Proyecto/Obstaculos/BP/Obstaculo_Piedra.Obstaculo_Piedra_C" (Transformation|GetWorldTransform _middle) "Undefined" 0 0))
      (Rendering|Material|SetMaterial (Variables|/Game/Proyecto/Obstaculos/BP/Obstaculo_Piedra.Obstaculo_Piedra_C|GetCube _returnvalue_2) 0 "/Game/Proyecto/Obstaculos/Assets/Obstaculo1_rocas/Obstaculo_Piedras_mat_2.Obstaculo_Piedras_mat_2"))
    (:1
      (Game|SpawnActorfromClass "/Game/Proyecto/Props/Carril_Moneda.Carril_Moneda_C" (Transformation|GetWorldTransform _middle) "Undefined" 0 0))
    (:2
      (Game|SpawnActorfromClass "/Game/Proyecto/Props/Oxigeno.Oxigeno_C" (Transformation|GetWorldTransform _middle) "Undefined" 0 0))
    (:3
      (Game|SpawnActorfromClass "/Game/Proyecto/Obstaculos/BP/Obstaculo_Cactus.Obstaculo_Cactus_C" (Transformation|GetWorldTransform _middle) "Undefined" 0 0))
    (:4
      (Game|SpawnActorfromClass "/Game/Proyecto/Obstaculos/BP/Obstaculo_Agacharse.Obstaculo_Agacharse_C" _returnvalue "Undefined" 0 0)
      (switch int (Math|Random|RandomIntegerinRange 0 2)
        (:0
          (Game|SpawnActorfromClass "/Game/Proyecto/Props/Carril_Moneda_Oxigeno.Carril_Moneda_Oxigeno_C" _returnvalue "Undefined" 0 0))
        (:1
          (Game|SpawnActorfromClass "/Game/Proyecto/Props/Carril_Moneda.Carril_Moneda_C" _returnvalue "Undefined" 0 0))
        (:2
          (Game|SpawnActorfromClass "/Game/Proyecto/Props/Carril_Moneda_XL.Carril_Moneda_XL_C" _returnvalue "Undefined" 0 0))))
    (:5
      (Game|SpawnActorfromClass "/Game/Proyecto/Props/Carril_Moneda.Carril_Moneda_C" (Transformation|GetWorldTransform _middle) "Undefined" 0 0))
    (:6
      (Game|SpawnActorfromClass "/Game/Proyecto/Obstaculos/BP/Obstaculo_Cactus.Obstaculo_Cactus_C" (Transformation|GetWorldTransform _middle) "Undefined" 0 0))
    (:7
      (Game|SpawnActorfromClass "/Game/Proyecto/Props/Gemas.Gemas_C" (Transformation|GetWorldTransform _middle) "Undefined" 0 0))
    (:8
      (Game|SpawnActorfromClass "/Game/Proyecto/PowerUps/BP/Iman.Iman_C" (Transformation|GetWorldTransform _middle) "Undefined" 0 0))
    (:9
      (Game|SpawnActorfromClass "/Game/Proyecto/PowerUps/BP/Desfasador.Desfasador_C" (Transformation|GetWorldTransform _middle) "Undefined" 0 0))))

(fn SpawnObstacleRight
  (bind _rigth (Variables|Default|GetRigth))
  (bind _returnvalue (Transformation|GetWorldTransform _rigth))
  (bind _returnvalue_2 (Transformation|GetWorldTransform _rigth))
  ;[1 1 1] Derecha
  (switch int (Math|Random|RandomIntegerinRange 0 (Variables|Default|GetMax_Rand_Obstacle))
    (:0
      (Game|SpawnActorfromClass "/Game/Proyecto/Obstaculos/BP/Obstaculo_Agacharse.Obstaculo_Agacharse_C" _returnvalue "Undefined" 0 0)
      (switch int (Math|Random|RandomIntegerinRange 0 3)
        (:0
          (Game|SpawnActorfromClass "/Game/Proyecto/Props/Carril_Moneda_Oxigeno.Carril_Moneda_Oxigeno_C" _returnvalue "Undefined" 0 0))
        (:1
          (Game|SpawnActorfromClass "/Game/Proyecto/Props/Carril_Moneda_XL.Carril_Moneda_XL_C" _returnvalue "Undefined" 0 0))
        (:2
          (Game|SpawnActorfromClass "/Game/Proyecto/Props/Gemas.Gemas_C" _returnvalue "Undefined" 0 0))
        (:3
          (Game|SpawnActorfromClass "/Game/Proyecto/PowerUps/BP/Iman.Iman_C" _returnvalue "Undefined" 0 0))))
    (:1
      (bind _returnvalue_3 (Game|SpawnActorfromClass "/Game/Proyecto/Obstaculos/BP/Obstaculo_Piedra.Obstaculo_Piedra_C" (Transformation|GetWorldTransform _rigth) "Undefined" 0 0))
      (Rendering|Material|SetMaterial (Variables|/Game/Proyecto/Obstaculos/BP/Obstaculo_Piedra.Obstaculo_Piedra_C|GetCube _returnvalue_3) 0 "/Game/Proyecto/Obstaculos/Assets/Obstaculo1_rocas/Obstaculo_Piedras_mat_2.Obstaculo_Piedras_mat_2"))
    (:2
      (Game|SpawnActorfromClass "/Game/Proyecto/Obstaculos/BP/Obstaculo_Cactus.Obstaculo_Cactus_C" (Transformation|GetWorldTransform _rigth) "Undefined" 0 0))
    (:3
      (Game|SpawnActorfromClass "/Game/Proyecto/PowerUps/BP/Desfasador.Desfasador_C" (Transformation|GetWorldTransform _rigth) "Undefined" 0 0))
    (:4
      (Game|SpawnActorfromClass "/Game/Proyecto/Props/Carril_Moneda_Oxigeno.Carril_Moneda_Oxigeno_C" _returnvalue_2 "Undefined" 0 0)
      (switch int (Math|Random|RandomIntegerinRange 0 3)
        (:0
          (Game|SpawnActorfromClass "/Game/Proyecto/Props/Carril_Moneda_Oxigeno.Carril_Moneda_Oxigeno_C" _returnvalue_2 "Undefined" 0 0))
        (:1
          (Game|SpawnActorfromClass "/Game/Proyecto/Props/Carril_Moneda_XL.Carril_Moneda_XL_C" _returnvalue_2 "Undefined" 0 0))
        (:2
          (Game|SpawnActorfromClass "/Game/Proyecto/Props/Gemas.Gemas_C" _returnvalue_2 "Undefined" 0 0))))
    (:5
      (Game|SpawnActorfromClass "/Game/Proyecto/Props/Oxigeno.Oxigeno_C" (Transformation|GetWorldTransform _rigth) "Undefined" 0 0))
    (:6
      (Game|SpawnActorfromClass "/Game/Proyecto/Obstaculos/BP/Gusano1-Derecha.Gusano1-Derecha_C" (Transformation|GetWorldTransform _rigth) "Undefined" 0 0))
    (:7
      (Game|SpawnActorfromClass "/Game/Proyecto/Props/Gemas.Gemas_C" (Transformation|GetWorldTransform _rigth) "Undefined" 0 0))
    (:8
      (Game|SpawnActorfromClass "/Game/Proyecto/PowerUps/BP/Escudo.Escudo_C" (Transformation|GetWorldTransform _rigth) "Undefined" 0 0))
    (:9
      (Game|SpawnActorfromClass "/Game/Proyecto/Obstaculos/BP/Gusano1-Izquierda.Gusano1-Izquierda_C" (Transformation|GetWorldTransform _rigth) "Undefined" 0 0))))

(fn SpawnSaltoMonedas
  (switch int (Math|Random|RandomIntegerinRange 0 2)
    (:0
      (Game|SpawnActorfromClass "/Game/Proyecto/Props/Carril_Moneda_Salto.Carril_Moneda_Salto_C" (Transformation|GetWorldTransform (Variables|Default|GetRigth)) "Undefined" 0 0))
    (:1
      (Game|SpawnActorfromClass "/Game/Proyecto/Props/Carril_Moneda_Salto.Carril_Moneda_Salto_C" (Transformation|GetWorldTransform (Variables|Default|GetMiddle)) "Undefined" 0 0))
    (:2
      (Game|SpawnActorfromClass "/Game/Proyecto/Props/Carril_Moneda_Salto.Carril_Moneda_Salto_C" (Transformation|GetWorldTransform (Variables|Default|GetLeft)) "Undefined" 0 0))))