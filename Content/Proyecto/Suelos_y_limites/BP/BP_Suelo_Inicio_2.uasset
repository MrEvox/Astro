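; BP_Suelo_Inicio_2 is a starting floor segment for what appears to be an endless runner with an astronaut.
; When an Astronauta overlaps its Collision, it has the game mode spawn the next floor via SpawnSuelo2 and adds multiplier-scaled race points.
; It also calls Breath on the player and slightly raises their clamped walk speed, then destroys itself after a short delay.
; Its obstacle and object spawn functions are empty.
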(event OnComponentBeginOverlap(Collision)
  (params (OverlappedComponent :type Primitive%20Component%20Object%20Reference) (OtherActor :type Actor%20Object%20Reference) (OtherComp :type Primitive%20Component%20Object%20Reference) (OtherBodyIndex :type Integer) (bFromSweep :type Boolean) (SweepResult :type Hit%20Result%20Structure%20%28by%20ref%29))
  (Utilities|Casting|CastToAstronauta OtherActor)
  (bind _asthird_person_game_mode (Utilities|Casting|CastToThirdPersonGameMode (Game|GetGameMode)))
  (Default|SpawnSuelo2 _asthird_person_game_mode)
  (bind _asthird_person_game_mode_2 (Utilities|Casting|CastToThirdPersonGameMode (Game|GetGameMode)))
  (Variables|/Game/ThirdPersonBP/Blueprints/ThirdPersonGameMode.ThirdPersonGameMode_C|SetPuntosCarrera _asthird_person_game_mode_2 (+ (* 1 (Variables|/Game/ThirdPersonBP/Blueprints/ThirdPersonGameMode.ThirdPersonGameMode_C|GetMultiplicador_puntos _asthird_person_game_mode_2)) (Variables|/Game/ThirdPersonBP/Blueprints/ThirdPersonGameMode.ThirdPersonGameMode_C|GetPuntosCarrera _asthird_person_game_mode_2)))
  (bind _asastronauta (Utilities|Casting|CastToAstronauta (Game|GetPlayerCharacter 0)))
  (Default|Breath _asastronauta)
  (bind _asastronauta_2 (Utilities|Casting|CastToAstronauta (Game|GetPlayerCharacter 0)))
  (Variables|/Script/Engine.CharacterMovementComponent|SetMaxWalkSpeed (Variables|/Script/Engine.Character|GetCharacterMovement _asastronauta_2) (Math|Float|Clamp(Float) (* 1.0025 (Variables|/Script/Engine.CharacterMovementComponent|GetMaxWalkSpeed (Variables|/Script/Engine.Character|GetCharacterMovement _asastronauta_2))) 1e+03 5e+03))
  (Utilities|FlowControl|Delay 0.8)
  (Actor|DestroyActor))

(event EventBeginPlay)

(event Collision|EventActorBeginOverlap
  (params (OtherActor :type Actor%20Object%20Reference)))

(event EventTick
  (params (DeltaSeconds :type Float%20%28single-precision%29)))

(fn ConstructionScript)

(fn SetSpawn)

(fn SpawnObstacle)

(fn SpawnObjetos)