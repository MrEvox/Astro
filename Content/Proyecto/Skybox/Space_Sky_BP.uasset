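; Space skybox actor that surrounds the player with a starry space backdrop.
; Every tick it teleports the Skybox component to the Astronauta player capsule's location so the player never reaches its edge.
; The construction script applies the space material and writes the actor's power, scene brightness and star brightness variables into the Spaces_Parameters material parameter collection.
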(event EventBeginPlay)

(event Collision|EventActorBeginOverlap
  (params (OtherActor :type Actor%20Object%20Reference)))

(event EventTick
  (params (DeltaSeconds :type Float%20%28single-precision%29))
  ;[5.177e+15 1 1] Actualizamos constantemente la posicion de la Skybox para que el jugador no llegue al final
  (bind _asastronauta (Utilities|Casting|CastToAstronauta (Game|GetPlayerCharacter 0)))
  (Transformation|SetWorldLocation (Variables|Default|GetSkybox) (Transformation|GetWorldLocation (Variables|/Script/Engine.Character|GetCapsuleComponent _asastronauta)) false true))

(fn ConstructionScript
  (Rendering|Material|SetMaterial (Variables|Default|GetSkybox) 0 (Variables|Default|GetSapce))
  (Rendering|Material|SetScalarParameterValue "/Game/Proyecto/Skybox/Spaces_Parameters.Spaces_Parameters" "Power" (Variables|Default|GetPower) :!class /Script/Engine.KismetMaterialLibrary)
  (Rendering|Material|SetScalarParameterValue "/Game/Proyecto/Skybox/Spaces_Parameters.Spaces_Parameters" "Brillo Escecna" (Variables|Default|GetBrillo%20Scena) :!class /Script/Engine.KismetMaterialLibrary)
  (Rendering|Material|SetScalarParameterValue "/Game/Proyecto/Skybox/Spaces_Parameters.Spaces_Parameters" "Brillo Estrellas" (Variables|Default|GetBrillo_strella) :!class /Script/Engine.KismetMaterialLibrary))